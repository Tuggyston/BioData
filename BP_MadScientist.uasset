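; Mad Scientist boss that moves along the X axis, hunting and shooting the player.
; Each Tick it checks line of sight, then patrols, chases or fires projectiles by distance, using line traces to turn or jump at walls and gaps.
; Any hit costs health, which advances its phase.
; From phase two it spawns enemy spawners, with a delayed destroy; phase three only sets the phase number.
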(event `self.ReceiveBeginPlay`
  (`KismetSystemLibrary.K2_SetTimer` self "SetCanSeePlayer" 2.0 true)
  (if (`self.canSpawnEnemies`)
    (`KismetSystemLibrary.K2_SetTimer` self "ResetEnemySpawner" 15.0 true)))

(event `self.ReceiveTick`
  (params (DeltaSeconds :type "Float (single-precision)"))
  (bind (_returnvalue_x _returnvalue_y _returnvalue_z) (`KismetMathLibrary.BreakVector` (`self.K2_GetActorLocation`)))
  (bind (_returnvalue_x_2 _returnvalue_y_2 _returnvalue_z_2) (`KismetMathLibrary.BreakVector` (`self.K2_GetActorLocation` (`GameplayStatics.GetPlayerPawn` 0))))
  (`parent.ReceiveTick` DeltaSeconds)
  (`self.UpdatePhase`)
  (`self.SetCanSeePlayer`)
  (if (not (`self.canSeePlayer`))
    (`self.Find Player`))
  (if (< (`self.MaxShootDistance`) (- (+ _returnvalue_x _returnvalue_z) (+ _returnvalue_x_2 _returnvalue_z_2)))
    (`self.ChasePlayer`)
    (else
      (`self.shootAtPlayer`)))
  (`self.CanWalk`)
  (if (`self.canSpawnEnemies`)
    (bind _actor (`self.SpawnEnemies`))
    (`KismetSystemLibrary.Delay` 10.0)
    (`self.K2_DestroyActor` _actor)))

(event `self.ReceiveActorBeginOverlap`
  (params (OtherActor :type "Actor Object Reference")))

(event `self.ReceiveHit`
  (params (MyComp :type "PrimitiveComponent Object Reference") (Other :type "Actor Object Reference") (OtherComp :type "PrimitiveComponent Object Reference") (bSelfMoved :type Boolean) (HitLocation :type "Vector Structure") (HitNormal :type "Vector Structure") (NormalImpulse :type "Vector Structure") (Hit :type "HitResult Structure (by ref)"))
  (set `self.Health` (- (`self.Health`) 10)))

(fn `CanJumpUp`
  (bind _returnvalue (`SceneComponent.K2_GetComponentLocation` (`self.Arrow1`)))
  (bind _returnvalue_2 (`SceneComponent.K2_GetComponentLocation` (`self.Arrow1`)))
  (bind _returnvalue_3 (+ (`SceneComponent.K2_GetComponentLocation` (`self.Arrow1`)) (0.0 0.0 200.0)))
  (bind _returnvalue_4 (+ (`SceneComponent.K2_GetComponentLocation` (`self.Arrow1`)) (0.0 0.0 200.0)))
  (bind _outactors (`GameplayStatics.GetAllActorsOfClass` "/Game/2DSideScrollerBP/Player/Projectiles/BP_Projectile_Test.BP_Projectile_Test_C"))
  (if (`self.canMoveRight`)
    (bind _outhit (`KismetSystemLibrary.LineTraceSingle` _returnvalue_3 (+ _returnvalue_3 (250.0 0.0 0.0)) "TraceTypeQuery1" false _outactors "ForDuration"))
    (bind (_outhit_2 _returnvalue_5) (`KismetSystemLibrary.LineTraceSingle` :`Start` _returnvalue :`End` (+ _returnvalue (50.0 0.0 0.0)) :`TraceChannel` "TraceTypeQuery1" :`DrawDebugType` "ForDuration"))
    (if (and (not _returnvalue_5) (`GameplayStatics.BreakHitResult` _outhit))
      (set `self.Jump?` true)
      (else
        (set `self.Jump?` false)))
    (else
      (bind _outhit_3 (`KismetSystemLibrary.LineTraceSingle` _returnvalue_4 (+ _returnvalue_4 (-250.0 0.0 0.0)) "TraceTypeQuery1" false _outactors "ForDuration"))
      (bind (_outhit_4 _returnvalue_6) (`KismetSystemLibrary.LineTraceSingle` :`Start` _returnvalue_2 :`End` (+ _returnvalue_2 (-50.0 0.0 0.0)) :`TraceChannel` "TraceTypeQuery1" :`DrawDebugType` "ForDuration"))
      (if (and (not _returnvalue_6) (`GameplayStatics.BreakHitResult` _outhit_3))
        (set `self.Jump?` true)
        (else
          (set `self.Jump?` false))))))

(fn `CanWalk`
  (bind _returnvalue (`SceneComponent.K2_GetComponentLocation` (`self.Arrow1`)))
  (bind _returnvalue_2 (`SceneComponent.K2_GetComponentLocation` (`self.Arrow1`)))
  (bind _outactors (`GameplayStatics.GetAllActorsOfClass` "/Game/2DSideScrollerBP/Player/Projectiles/BP_Projectile_Test.BP_Projectile_Test_C"))
  (if (`self.canMoveRight`)
    (bind _outhit (`KismetSystemLibrary.LineTraceSingle` _returnvalue (- _returnvalue (0.0 0.0 150.0)) "TraceTypeQuery1" false _outactors))
    (if (not (`GameplayStatics.BreakHitResult` _outhit))
      (`self.Jump`))
    (else
      (bind _outhit_2 (`KismetSystemLibrary.LineTraceSingle` _returnvalue_2 (- _returnvalue_2 (0.0 0.0 150.0)) "TraceTypeQuery1" false _outactors))
      (if (not (`GameplayStatics.BreakHitResult` _outhit_2))
        (`self.Jump`)))))

(fn `ChasePlayer`
  (bind _returnvalue_x (`KismetMathLibrary.BreakVector` (`self.K2_GetActorLocation`)))
  (bind _returnvalue_x_2 (`KismetMathLibrary.BreakVector` (`self.K2_GetActorLocation` (`GameplayStatics.GetPlayerPawn` 0))))
  (if (< _returnvalue_x _returnvalue_x_2)
    (`self.K2_SetActorRotation` (struct))
    (`self.AddMovementInput` (5.0 0.0 0.0) 10.0)
    (else
      (`self.K2_SetActorRotation` (struct :`Yaw` 180.0))
      (`self.AddMovementInput` (-5.0 0.0 0.0))))
  (`self.CanJumpUp`)
  (if (`self.Jump?`)
    (`self.Jump`)
    (set `self.Jump?` false)
    (`self.SetCanSeePlayer`)
    (if (`self.canSeePlayer`)
      (`self.Find Player`))))

(fn `Check Movement`
  (set `self.LastLocation` (`self.K2_GetActorLocation`))
  (if (== (`KismetMathLibrary.VSize` (`self.LastLocation`)) (`KismetMathLibrary.VSize` (`self.K2_GetActorLocation`)))
    (if (`self.canMoveRight`)
      (set `self.canMoveRight` false)
      (set `self.canMoveLeft` true)
      (elif (`self.canMoveLeft`)
        (set `self.canMoveRight` true)
        (set `self.canMoveLeft` false)))))

(fn `Find Player`
  (bind _returnvalue_x (`KismetMathLibrary.BreakVector` (`self.K2_GetActorLocation`)))
  (bind _returnvalue_x_2 (`KismetMathLibrary.BreakVector` (`self.K2_GetActorLocation` (`GameplayStatics.GetPlayerPawn` 0))))
  ;[1 1 1] If Player out of shooting distance find player
  (if (>= (`KismetMathLibrary.VSize` (- (`self.K2_GetActorLocation` (`GameplayStatics.GetPlayerPawn` 0)) (`self.K2_GetActorLocation`))) (`self.MaxShootDistance`))
    ;[1 1 1] Call move direction function and add movement in the direction calculated
    (`self.Move Direction`)
    (if (`self.canMoveRight`)
      (`self.K2_SetActorRotation` (struct))
      (`self.AddMovementInput` (5.0 0.0 0.0))
      (elif (`self.canMoveLeft`)
        (`self.K2_SetActorRotation` (struct :`Yaw` 180.0))
        (`self.AddMovementInput` (-5.0 0.0 0.0))))
    (elif (< _returnvalue_x _returnvalue_x_2)
      (`self.K2_SetActorRotation` (struct))
      (else
        (`self.K2_SetActorRotation` (struct :`Yaw` 180.0))))))

(fn `Move Direction`
  (bind _jump_ (`self.Jump?`))
  (bind _arrow1 (`self.Arrow1`))
  (bind _returnvalue (`SceneComponent.K2_GetComponentLocation` _arrow1))
  (bind _returnvalue_2 (`SceneComponent.K2_GetComponentLocation` _arrow1))
  (bind _returnvalue_3 (`NavMovementComponent.IsFalling` (`self.CharacterMovement`)))
  (if (`self.canMoveRight`)
    ;[1 1 1] Test which direction can move
    (bind _outactors (`GameplayStatics.GetAllActorsOfClass` "/Game/2DSideScrollerBP/Player/Projectiles/BP_Projectile_Test.BP_Projectile_Test_C"))
    (bind _outhit (`KismetSystemLibrary.LineTraceSingle` _returnvalue (+ _returnvalue (150.0 0.0 0.0)) "TraceTypeQuery1" false _outactors "ForDuration" true (struct :`R` 1.0 :`A` 1.0) (struct :`G` 1.0 :`A` 1.0) 0.2))
    (if (`GameplayStatics.BreakHitResult` _outhit)
      ;[1 1 1] check if jumping or falling before allowing boss to turn
      (if (not (`NavMovementComponent.IsFalling` (`self.CharacterMovement`)))
        (`self.CanJumpUp`))
      (if _jump_
        (set `self.canMoveRight` true)
        (elif (not _returnvalue_3)
          ;[1 1 1] Set Direction when line trace hit
          (set `self.canMoveRight` false)
          (set `self.canMoveLeft` true))))
    (else
      (`GameplayStatics.GetAllActorsOfClass` "/Game/2DSideScrollerBP/Player/Projectiles/BP_Projectile_Test.BP_Projectile_Test_C")
      (bind _outhit_2 (`KismetSystemLibrary.LineTraceSingle` _returnvalue_2 (+ _returnvalue_2 (-150.0 0.0 0.0)) "TraceTypeQuery1" false _outactors "ForDuration" true (struct :`R` 1.0 :`A` 1.0) (struct :`G` 1.0 :`A` 1.0) 0.2))
      (if (`GameplayStatics.BreakHitResult` _outhit_2)
        (if (not (`NavMovementComponent.IsFalling` (`self.CharacterMovement`)))
          (`self.CanJumpUp`))
        (if _jump_
          (set `self.canMoveLeft` true)
          (elif (not _returnvalue_3)
            (set `self.canMoveLeft` false)
            (set `self.canMoveRight` true)))))))

(fn `ResetEnemySpawner`
  (set `self.canSpawnEnemies` true))

(fn `Set Shoot Rotation`
  (returns (Transform :type "Transform Structure"))
  (return (`KismetMathLibrary.MakeTransform` (+ (`self.K2_GetActorLocation`) (-100.0 -100.0 0.0)) (`KismetMathLibrary.MakeRotator` (* (+ (.roll (`KismetMathLibrary.MakeRotFromX` (* (`KismetMathLibrary.RotateAngleAxis` (`self.GetActorForwardVector`) 0.0 (0.0 1.0 0.0)) 1000.0))) (.roll (`self.K2_GetActorRotation`))) -1.0) (+ (.pitch (`KismetMathLibrary.MakeRotFromX` (* (`KismetMathLibrary.RotateAngleAxis` (`self.GetActorForwardVector`) 0.0 (0.0 1.0 0.0)) 1000.0))) (.pitch (`self.K2_GetActorRotation`))) (+ (.yaw (`KismetMathLibrary.MakeRotFromX` (* (`KismetMathLibrary.RotateAngleAxis` (`self.GetActorForwardVector`) 0.0 (0.0 1.0 0.0)) 1000.0))) (.yaw (`self.K2_GetActorRotation`)))))))

(fn `SetCanSeePlayer`
  (bind _outhit (`KismetSystemLibrary.LineTraceSingle` :`Start` (`self.K2_GetActorLocation`) :`End` (`self.K2_GetActorLocation` (`GameplayStatics.GetPlayerPawn` 0)) :`TraceChannel` "TraceTypeQuery1" :`DrawTime` 1.0))
  (if (== (`.HitActor` (`GameplayStatics.BreakHitResult` _outhit)) (`GameplayStatics.GetPlayerPawn` 0))
    (set `self.canSeePlayer` true)
    (else
      (set `self.canSeePlayer` false))))

(fn `shootAtPlayer`
  ;[1 1 1] Shoot if canSeePlayer and is within a specific distance from the player
  (if (`self.canSeePlayer`)
    (if (not (`NavMovementComponent.IsFalling` (`self.CharacterMovement`)))
      (if (<= (`KismetMathLibrary.VSize` (- (`self.K2_GetActorLocation`) (`self.K2_GetActorLocation` (`GameplayStatics.GetPlayerPawn` 0)))) (`self.MaxShootDistance`))
        (`|SpawnActorFromClass` "/Game/2DSideScrollerBP/Player/Projectiles/BP_Projectile_Test.BP_Projectile_Test_C" (`KismetMathLibrary.MakeTransform` (+ (`SceneComponent.K2_GetComponentLocation` (`self.Arrow1`)) (10.0 0.0 0.0)) (`KismetMathLibrary.FindLookAtRotation` (`self.K2_GetActorLocation`) (`self.K2_GetActorLocation` (`GameplayStatics.GetPlayerPawn` 0)))) "AlwaysSpawn" "OverrideRootScale" self null)))))

(fn `SpawnEnemies`
  (returns (Actor :type "Actor Object Reference"))
  (if (`self.canSpawnEnemies`)
    (bind _returnvalue (`|SpawnActorFromClass` "/Game/EnemySpawner/BP_EnemySpawner.BP_EnemySpawner_C" (`KismetMathLibrary.Conv_VectorToTransform` (+ (`self.K2_GetActorLocation`) (50.0 0.0 0.0))) "Undefined" "OverrideRootScale" null null))
    (set `self.canSpawnEnemies` false)
    (return _returnvalue)))

(fn `UpdatePhase`
  ;[1 1 1] Change phases depending on current health
  (if (<= (`self.Health`) 60)
    (set `self.phase` 2)
    (set `self.canSpawnEnemies` true)
    (if (<= (`self.Health`) 30)
      (set `self.phase` 3))))

(fn `UserConstructionScript`
  (`parent.UserConstructionScript`))