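; Object spawner that places item and special weapon pickups in the level.
; On BeginPlay, WhichItem resets EnemiesKilled and spawns ItemClass at an X offset from the player; its random roll always passes and the kill-count check is unused.
; While CanSpawn is true, Tick spawns BP_SpecialWeapon at the spawner's location until ObjectSpawned, which this Blueprint never sets.
; Once ObjectSpawned is true, Tick clears CanSpawn and destroys the spawner if HasPickup.
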(event `self.ReceiveBeginPlay`
  (`self.WhichItem?`))

(event `self.ReceiveTick`
  (params (DeltaSeconds :type "Float (single-precision)"))
  (if (`self.CanSpawn`)
    (if (`self.ObjectSpawned?`)
      (set `self.CanSpawn` false)
      (if (`self.hasPickup?`)
        (`self.K2_DestroyActor`))
      (else
        (`|SpawnActorFromClass` "/Game/ObjectSpawners_BP/BP_SpecialWeapon.BP_SpecialWeapon_C" (`KismetMathLibrary.Conv_VectorToTransform` (`self.K2_GetActorLocation`)) "Undefined" "OverrideRootScale" null null)))))

(event `self.ReceiveActorBeginOverlap`
  (params (OtherActor :type "Actor Object Reference")))

(fn `UserConstructionScript`)

(fn `WhichItem?`
  (if true
    (set `self.enemiesKilled` 0)
    (if (<= (`KismetMathLibrary.RandomIntegerInRange` 0 100) 100)
      (`|SpawnActorFromClass` (`self.ItemClass`) (`KismetMathLibrary.MakeTransform` (+ (`self.K2_GetActorLocation` (`GameplayStatics.GetPlayerPawn` 0)) (1500.0 0.0 0.0))) "Undefined" "OverrideRootScale" null null))))