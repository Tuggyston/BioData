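; Spawned world object that settles onto the ground and can be destroyed by hits from the Kraken boss.
; On BeginPlay it caches the first BP_Kraken_Boss, then traces downward and moves just above the hit point.
; If the trace hits Base_Enemy it nudges along X and retries, accepting the last location when attempts run out.
; HitBox hits from that boss decrement Damage, which serves as remaining health, and zero destroys the actor.
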(event `Check For Death`
  (if (== (`self.Damage`) 0)
    (`self.K2_DestroyActor`)))

(event `self.Hit Box.OnComponentHit`
  (params (HitComponent :type "PrimitiveComponent Object Reference") (OtherActor :type "Actor Object Reference") (OtherComp :type "PrimitiveComponent Object Reference") (NormalImpulse :type "Vector Structure") (Hit :type "HitResult Structure (by ref)"))
  (if (== OtherActor (`self.Object Hit Reference`))
    (set `self.Damage` (- (`self.Damage`) 1))
    (`self.Check For Death`)))

(event `self.ReceiveBeginPlay`
  (bind _returnvalue (`self.K2_GetActorLocation`))
  ;[1 1 1] When spawned object is spawned, looks for the ground, if it finds an enemy, retrys at a slightly new location. After 3 attempts, it just accepts current faulty location
  (bind _outactors (`GameplayStatics.GetAllActorsOfClass` "/Game/2DSideScrollerBP/Bosses/BP_Kraken_Boss.BP_Kraken_Boss_C"))
  (set `self.Object Hit Reference` (`|GetArrayItem` _outactors))
  (for _index (range (+ (`self.Last Index`) 1)) :!label _label
    (set `self.Index` _index)
    (bind (_outhit _returnvalue_2) (`KismetSystemLibrary.LineTraceSingle` :`Start` _returnvalue :`End` (`KismetMathLibrary.MakeVector` (.x _returnvalue) (.y _returnvalue) -5000.0) :`TraceChannel` "TraceTypeQuery1" :`DrawDebugType` "Persistent"))
    (bind (_bblockinghit _binitialoverlap _time _distance _location _impactpoint _normal _impactnormal _physmat _hitactor) (`GameplayStatics.BreakHitResult` _outhit))
    (set `self.Hit Location` _location)
    (set `self.Hit Actor` _hitactor)
    (if (!= (`self.Hit Actor`) "/Game/2DSideScrollerBP/Enemies/Base_Enemy.Base_Enemy")
      (`self.Move Down` _returnvalue_2)
      (`self.BreakLoop`)
      (else
        (`self.K2_SetActorLocation` (`KismetMathLibrary.MakeVector` (+ (.x (`self.K2_GetActorLocation`)) 10.0) (.y (`self.K2_GetActorLocation`)) (.z (`self.K2_GetActorLocation`))))
        (if (== (`self.Index`) (`self.Last Index`))
          (`self.Move Down` false))))))

(event `BreakLoop`
  ;[1 1 1] When spawned object is spawned, looks for the ground, if it finds an enemy, retrys at a slightly new location. After 3 attempts, it just accepts current faulty location
  (goto _label :!via `Break`))

(fn `Move Down`
  (params (Teleport :type Boolean))
  ;[1 1 1] Sets acotrs location to hit location
  (`self.K2_SetActorLocation` self (+ (`self.Hit Location`) (0.0 0.0 100.0)) false Teleport))

(fn `UserConstructionScript`)