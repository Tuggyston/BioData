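; BP_Stalagmite is a flipbook-based stalagmite obstacle that shatters when the Kraken boss hits it.
; On BeginPlay it caches the first BP_Kraken_Boss in the level, loops its flipbook, and uses a downward line trace to place itself at a fixed height above the hit surface.
; When the Kraken overlaps its Box, it plays the broken flipbook once, then destroys itself after that animation and an extra delay.
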(event `self.ReceiveBeginPlay`
  (bind _returnvalue (`self.K2_GetActorLocation`))
  (bind _outactors (`GameplayStatics.GetAllActorsOfClass` "/Game/2DSideScrollerBP/Bosses/BP_Kraken_Boss.BP_Kraken_Boss_C"))
  (set `self.Kraken` (`|GetArrayItem` _outactors))
  (`PaperFlipbookComponent.SetLooping` (`self.Stalagmite`) true)
  (bind _outhit (`KismetSystemLibrary.LineTraceSingle` _returnvalue (+ _returnvalue (0.0 0.0 -10000.0)) "TraceTypeQuery1"))
  (`self.K2_SetActorLocation` (+ (`.Location` (`GameplayStatics.BreakHitResult` _outhit)) (0.0 0.0 450.0))))

(event `self.Box.OnComponentBeginOverlap`
  (params (OverlappedComponent :type "PrimitiveComponent Object Reference") (OtherActor :type "Actor Object Reference") (OtherComp :type "PrimitiveComponent Object Reference") (OtherBodyIndex :type Integer) (bFromSweep :type Boolean) (SweepResult :type "HitResult Structure (by ref)"))
  (bind _stalagmite (`self.Stalagmite`))
  (if (== OtherActor (`self.Kraken`))
    (`PaperFlipbookComponent.SetFlipbook` _stalagmite "/Game/Levels/Blueprints/Stalagmites/FB_StalagmiteBroken.FB_StalagmiteBroken")
    (`PaperFlipbookComponent.SetLooping` _stalagmite false)
    (`KismetSystemLibrary.Delay` (+ (`PaperFlipbookComponent.GetFlipbookLength` _stalagmite) 5.0))
    (`KismetSystemLibrary.PrintString` "after")
    (`self.K2_DestroyActor`)))

(fn `UserConstructionScript`)