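; Manager actor that periodically spawns BP_Stalagmite hazards at an offset from the water player character.
; BeginPlay starts a looping SpawnStalagmite timer, rolling its random interval only once.
; Each call looks up the first BP_PlayerCharacter_Water and, when Active, spawns only if it has moved since the last spawn.
; Stalagmites are enlarged and placed on the Y=0 plane, offset in X and Z.
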(event `self.ReceiveBeginPlay`
  (`KismetSystemLibrary.K2_SetTimer` null "SpawnStalagmite" (`KismetMathLibrary.RandomFloatInRange` (`self.spawnRateMin`) (`self.spawnRateMax`)) true))

(fn `SpawnStalagmite`
  (bind _returnvalue (`self.K2_GetActorLocation` (`self.Character`)))
  (bind _outactors (`GameplayStatics.GetAllActorsOfClass` "/Game/2DSideScrollerBP/Player/BP_PlayerCharacter_Water.BP_PlayerCharacter_Water_C"))
  (set `self.Character` (`|GetArrayItem` _outactors))
  (if (`self.active`)
    (if (not (== (`self.currentCharacterLocation`) _returnvalue))
      (`|SpawnActorFromClass` "/Game/Levels/Blueprints/BP_Stalagmite.BP_Stalagmite_C" (`KismetMathLibrary.MakeTransform` (`KismetMathLibrary.MakeVector` (+ (.x _returnvalue) (`self.X DistanceFromCharacter`)) 0.0 (+ (.z _returnvalue) (`self.Y DistanceFromCharacter`))) (struct) (5.0 5.0 5.0)) "Undefined" "OverrideRootScale" null null)
      (set `self.currentCharacterLocation` (`self.K2_GetActorLocation` (`self.Character`))))))

(fn `UserConstructionScript`)