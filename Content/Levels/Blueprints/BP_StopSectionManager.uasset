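; BP_StopSectionManager is a level trigger that holds the player in a timed enemy encounter.
; When the player overlaps StartBox, it spawns a BP_EnemySpawner at SpawnerLocation set to Guppy_Grunt, removes the trigger and switches two blocking boxes to BlockAll.
; After a delay of Time, it destroys the first BP_EnemySpawner found in the world, not a stored reference, then destroys itself.
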(event `self.StartBox.OnComponentBeginOverlap`
  (params (OverlappedComponent :type "PrimitiveComponent Object Reference") (OtherActor :type "Actor Object Reference") (OtherComp :type "PrimitiveComponent Object Reference") (OtherBodyIndex :type Integer) (bFromSweep :type Boolean) (SweepResult :type "HitResult Structure (by ref)"))
  (cast `/Game/2DSideScrollerBP/Player/BP_PlayerCharacter` OtherActor)
  (`self.Spawn Enemies`)
  (`ActorComponent.K2_DestroyComponent` (`self.StartBox`))
  (`PrimitiveComponent.SetCollisionProfileName` (`self.Blocking Box 1`) "BlockAll" true)
  (`PrimitiveComponent.SetCollisionProfileName` (`self.Blocking Box 2`) "BlockAll" true)
  (`KismetSystemLibrary.Delay` (`self.Time`))
  (bind _outactors (`GameplayStatics.GetAllActorsOfClass` "/Game/EnemySpawner/BP_EnemySpawner.BP_EnemySpawner_C"))
  (`self.K2_DestroyActor` (`|GetArrayItem` _outactors))
  (`self.K2_DestroyActor`))

(fn `Spawn Enemies`
  (bind _returnvalue (`|SpawnActorFromClass` "/Game/EnemySpawner/BP_EnemySpawner.BP_EnemySpawner_C" (`KismetMathLibrary.MakeTransform` (`SceneComponent.K2_GetComponentLocation` (`self.SpawnerLocation`))) "Undefined" "OverrideRootScale" null null))
  (set `/Game/EnemySpawner/BP_EnemySpawner.Class` "/Game/2DSideScrollerBP/Enemies/Guppy_Grunt.Guppy_Grunt_C" _returnvalue))

(fn `UserConstructionScript`)