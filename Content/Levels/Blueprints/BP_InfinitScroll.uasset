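; BP_InfinitScroll is a self-replicating level segment that extends an endless scroll as the water player character moves through it.
; When BP_PlayerCharacter_Water enters the Overlap component, it spawns another instance of its own class at SpawnPoint with a fixed, non-uniform scale.
; Beforehand it loops over existing instances to destroy the first, but the contradictory index checks mean that destroy never runs.
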(event `self.Overlap.OnComponentBeginOverlap`
  (params (OverlappedComponent :type "PrimitiveComponent Object Reference") (OtherActor :type "Actor Object Reference") (OtherComp :type "PrimitiveComponent Object Reference") (OtherBodyIndex :type Integer) (bFromSweep :type Boolean) (SweepResult :type "HitResult Structure (by ref)"))
  (bind _returnvalue (`GameplayStatics.GetObjectClass` self))
  (cast `/Game/2DSideScrollerBP/Player/BP_PlayerCharacter_Water` OtherActor)
  (bind _outactors (`GameplayStatics.GetAllActorsOfClass` _returnvalue))
  (for (_array_element _array_index) _outactors
    (if (< _array_index 1)
      _
      (elif (== _array_index 0)
        (`self.K2_DestroyActor` _array_element))))
  (`|SpawnActorFromClass` _returnvalue (`KismetMathLibrary.MakeTransform` (`SceneComponent.K2_GetComponentLocation` (`self.SpawnPoint`)) (struct) (3.25 1.0 3.25)) "Undefined" "OverrideRootScale" null null))

(fn `UserConstructionScript`)