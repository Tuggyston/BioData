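; BP_Button is a shootable switch that opens level doors two at a time in sequence.
; On BeginPlay it caches every BP_Door; a BP_BaseProjectile overlap or any damage triggers the press logic.
; When CurrentElm matches WhichDoors minus two, a custom ranged-loop macro flags the next doors as opened.
; Updated progress counters are copied to every BP_Button to keep the sequence in sync.
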(event `self.ReceiveBeginPlay`
  (bind _outactors (`GameplayStatics.GetAllActorsOfClass` "/Game/Levels/Level_3/ButtonDoor/BP_Door.BP_Door_C"))
  (bind _array_element (`self.MyForLoop` _outactors (`KismetArrayLibrary.Array_Length` _outactors))
    (:`Loop Body`
      (`KismetArrayLibrary.Array_Add` (`self.DoorArray`) _array_element))))

(event `self.ReceiveActorBeginOverlap`
  (params (OtherActor :type "Actor Object Reference"))
  (bind _currentelm (`self.currentElm`))
  ;[1 1 1] ButtonPress
  (if (== (`GameplayStatics.GetObjectClass` OtherActor) "/Game/2DSideScrollerBP/Player/Projectiles/BP_BaseProjectile.BP_BaseProjectile_C")
    (`KismetSystemLibrary.PrintString` "You hear a door open." :!label _label)
    (`self.K2_DestroyActor` OtherActor)
    (if (== _currentelm (- (`self.whichDoors`) 2)) :!label _label_2
      (bind _output_get (set `self.loopCounter` (+ (`self.loopCounter`) 2)))
      (bind _array_element (`self.MyForLoop` (`self.DoorArray`) _output_get _currentelm)
        (:`Loop Body`
          (set `/Game/Levels/Level_3/ButtonDoor/BP_Door.doorOpened` true _array_element)
          (set `self.currentElm` (+ (`self.currentElm`) 1))
          (bind _outactors (`GameplayStatics.GetAllActorsOfClass` "BP_Button_C"))
          (bind _array_element_2 (`self.MyForLoop` _outactors (`KismetArrayLibrary.Array_Length` _outactors))
            (:`Loop Body`
              (set `/Game/Levels/Level_3/ButtonDoor/BP_Button.currentElm` (`self.currentElm`) _array_element_2)
              (set `/Game/Levels/Level_3/ButtonDoor/BP_Button.loopCounter` (`self.loopCounter`) _array_element_2)
              (goto _label_2))))))))

(event `self.ReceiveAnyDamage`
  (params (Damage :type "Float (single-precision)") (DamageType :type "DamageType Object Reference") (InstigatedBy :type "Controller Object Reference") (DamageCauser :type "Actor Object Reference"))
  ;[1 1 1] ButtonPress
  (goto _label))

(fn `UserConstructionScript`)